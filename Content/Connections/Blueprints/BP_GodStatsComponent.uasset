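; BP_GodStatsComponent holds a god's Health, Followers, Faith and Connection and implements its actions against another god.
; Clamped add and remove functions back Pray, Smite, Sacrifice, Convert, Miracle and Defend, with Connection paying for the offensive ones.
; TakeFollowerDamage lowers Health, minus Defense while defending, and zero Health or Followers means defeat.
; ConvertFollowersFrom is empty, and Convert damages the caster while removing then re-adding the target's followers.
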(fn `AddConnection`
  (params (Amount :type Integer))
  (set `self.Connection` (`KismetMathLibrary.Clamp` (+ Amount (`self.Connection`)) 0 (`self.MaxConnection`))))

(fn `AddFaith`
  (params (Amount :type Integer))
  (set `self.Faith` (`KismetMathLibrary.Clamp` (+ Amount (`self.Faith`)) 0 (`self.MaxFaith`))))

(fn `AddFollowers`
  (params (Amount :type Integer))
  (set `self.Followers` (`KismetMathLibrary.Clamp` (+ Amount (`self.Followers`)) 0 (`self.MaxFollowers`))))

(fn `AddHealth`
  (params (Amount :type Integer))
  (set `self.Health` (`KismetMathLibrary.Clamp` (+ Amount (`self.Health`)) 0 (`self.MaxHealth`))))

(fn `Convert`
  (params (OtherGod :type "/Game/Connections/Blueprints/BP_GodStatsComponent Object Reference"))
  (returns (Successful :type Boolean))
  (bind _successful (`self.SpendConnection` 20))
  (if _successful
    (`self.TakeFollowerDamage` 6)
    (`self.RemoveConnection` OtherGod 10)
    (`self.RemoveFollowers` OtherGod 6)
    (`self.AddFollowers` OtherGod 6)
    (return true)
    (else
      (return false))))

(fn `ConvertFollowersFrom`
  (params (TargetGodStats :type "/Game/Connections/Blueprints/BP_GodStatsComponent Object Reference") (AmountToRemove :type Integer) (AmountToGain :type Integer)))

(fn `Defend`
  (set `self.IsDefending` true))

(fn `IsDefeated`
  (returns (IsDefeated :type Boolean))
  (return (or (<= (`self.Followers`) 0) (<= (`self.Health`) 0))))

(fn `Miracle`
  (params (OtherGod :type "/Game/Connections/Blueprints/BP_GodStatsComponent Object Reference"))
  (returns (Successful :type Boolean))
  (bind _successful (`self.SpendConnection` (`self.MiracleCost`)))
  (if _successful
    (`self.TakeFollowerDamage` OtherGod (* (`self.DivinePower`) 10))
    (return true)
    (else
      (return false))))

(fn `Pray`
  (`self.AddHealth` 5)
  (`self.AddConnection` 10))

(fn `RemoveConnection`
  (params (Amount :type Integer))
  (set `self.Connection` (`KismetMathLibrary.Clamp` (- (`self.Connection`) Amount) 0 (`self.MaxConnection`))))

(fn `RemoveFollowers`
  (params (Amount :type Integer))
  (set `self.Followers` (`KismetMathLibrary.Clamp` (- (`self.Followers`) Amount) 0 (`self.MaxFollowers`))))

(fn `RemoveHealth`
  (params (Amount :type Integer))
  (set `self.Health` (`KismetMathLibrary.Clamp` (- (`self.Health`) Amount) 0 (`self.MaxHealth`)))
  (`KismetSystemLibrary.PrintString` (`KismetStringLibrary.Concat_StrStr` (`KismetSystemLibrary.GetDisplayName` self) " -                          " (`KismetStringLibrary.Conv_IntToString` Amount)) true true (struct :`R` 0.066304 :`G` 1.0 :`B` 0.178192 :`A` 1.0)))

(fn `ResetTemporaryEffects`
  (`self.SetDefending` false))

(fn `Sacrifice`
  (`KismetSystemLibrary.PrintString` "Sacrifing")
  (`self.RemoveFollowers` 8)
  (`self.RemoveHealth` 10)
  (`self.AddConnection` 40))

(fn `SetDefending`
  (params (IsDefending :type Boolean))
  (set `self.IsDefending` IsDefending))

(fn `Smite`
  (params (OtherGod :type "/Game/Connections/Blueprints/BP_GodStatsComponent Object Reference"))
  (returns (Sucessful :type Boolean))
  (bind _returnvalue (+ (`self.DivinePower`) 8))
  (bind _successful (`self.SpendConnection` 3))
  (if _successful
    (`self.TakeFollowerDamage` OtherGod _returnvalue)
    (`self.RemoveConnection` OtherGod (* _returnvalue 1.5))
    (return true)
    (else
      (return false))))

(fn `SpendConnection`
  (params (Amount :type Integer))
  (returns (Successful :type Boolean))
  (if (>= (`self.Connection`) Amount)
    (set `self.Connection` (`KismetMathLibrary.Clamp` (- (`self.Connection`) Amount) 0 (`self.MaxConnection`)))
    (return true)
    (else
      (return false))))

(fn `SpendFaith`
  (params (Amount :type Integer))
  (returns (Successful :type Boolean))
  (bind _returnvalue (< Amount (`self.Faith`)))
  (if _returnvalue
    (set `self.Faith` (- (`self.Faith`) Amount)))
  (return _returnvalue))

(fn `TakeFollowerDamage`
  (params (Amount :type Integer))
  (if (`self.IsDefending`)
    (`self.RemoveHealth` (- Amount (`self.Defense`)))
    (else
      (`self.RemoveHealth` Amount))))

(fn `UnDefend`
  (set `self.IsDefending` false))
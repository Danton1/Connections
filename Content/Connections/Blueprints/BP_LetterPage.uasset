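; BP_LetterPage is a collectible letter page that the player picks up by interacting with it.
; Its collider shows a "Collect" prompt on overlapping actors that implement BPI_InteractActor and clears it when they leave.
; On Interact, it sends a "Page Collected!" speech message to the interacting actor, then destroys the collider and itself, without recording the pickup.
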(event `self.Collider.OnComponentBeginOverlap`
  (params (OverlappedComponent :type "PrimitiveComponent Object Reference") (OtherActor :type "Actor Object Reference") (OtherComp :type "PrimitiveComponent Object Reference") (OtherBodyIndex :type Integer) (bFromSweep :type Boolean) (SweepResult :type "HitResult Structure (by ref)"))
  (if (`KismetSystemLibrary.DoesImplementInterface` OtherActor "/Game/Connections/Interfaces/BPI_InteractActor.BPI_InteractActor_C")
    (message `/Game/Connections/Interfaces/BPI_InteractActor.SetInteractText` OtherActor "Collect")))

(event `self.Collider.OnComponentEndOverlap`
  (params (OverlappedComponent :type "PrimitiveComponent Object Reference") (OtherActor :type "Actor Object Reference") (OtherComp :type "PrimitiveComponent Object Reference") (OtherBodyIndex :type Integer))
  (if (`KismetSystemLibrary.DoesImplementInterface` OtherActor "/Game/Connections/Interfaces/BPI_InteractActor.BPI_InteractActor_C")
    (message `/Game/Connections/Interfaces/BPI_InteractActor.RemoveInteractText` OtherActor)))

(event `/Game/Connections/Interfaces/BPI_Interactable.Interact`
  (params (InteractActor :type "Actor Object Reference"))
  (message `/Game/Connections/Interfaces/BPI_InteractActor.SetSpeechText` InteractActor "Page Collected!")
  (`ActorComponent.K2_DestroyComponent` (`self.Collider`))
  (`self.K2_DestroyActor`))

(fn `UserConstructionScript`
  (`parent.UserConstructionScript`))
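; BP_NPC is a talkable NPC character that the player can interact with.
; Its InteractionCollider shows a "Talk" prompt on actors implementing BPI_InteractActor when they enter, and removes it when they leave.
; On Interact, it clears the prompt and displays a fixed greeting through the same interface, then removes it after a short delay.
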(event `self.InteractionCollider.OnComponentBeginOverlap`
  (params (OverlappedComponent :type "PrimitiveComponent Object Reference") (OtherActor :type "Actor Object Reference") (OtherComp :type "PrimitiveComponent Object Reference") (OtherBodyIndex :type Integer) (bFromSweep :type Boolean) (SweepResult :type "HitResult Structure (by ref)"))
  (if (`KismetSystemLibrary.DoesImplementInterface` OtherActor "/Game/Connections/Interfaces/BPI_InteractActor.BPI_InteractActor_C")
    (message `/Game/Connections/Interfaces/BPI_InteractActor.SetInteractText` OtherActor "Talk")))

(event `self.InteractionCollider.OnComponentEndOverlap`
  (params (OverlappedComponent :type "PrimitiveComponent Object Reference") (OtherActor :type "Actor Object Reference") (OtherComp :type "PrimitiveComponent Object Reference") (OtherBodyIndex :type Integer))
  (if (`KismetSystemLibrary.DoesImplementInterface` OtherActor "/Game/Connections/Interfaces/BPI_InteractActor.BPI_InteractActor_C")
    (message `/Game/Connections/Interfaces/BPI_InteractActor.RemoveInteractText` OtherActor)))

(event `/Game/Connections/Interfaces/BPI_Interactable.Interact`
  (params (InteractActor :type "Actor Object Reference"))
  (message `/Game/Connections/Interfaces/BPI_InteractActor.RemoveInteractText` InteractActor)
  (message `/Game/Connections/Interfaces/BPI_InteractActor.SetSpeechText` InteractActor "Hello There!")
  (`KismetSystemLibrary.Delay` 2.0)
  (message `/Game/Connections/Interfaces/BPI_InteractActor.RemoveSpeechText` InteractActor))

(fn `UserConstructionScript`)
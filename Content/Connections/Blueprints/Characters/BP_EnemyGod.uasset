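; BP_EnemyGod is an enemy character Blueprint that picks its intent at random.
; ChooseIntent casts a random index within the E_EnemyIntent entry count to that enum, with no weighting or state checks.
; GetIntentDescription returns an empty string, and PlayAnim plays a given animation directly on the skeletal mesh with optional looping.
; The event graph is empty, and construction only calls the parent script.
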(fn `ChooseIntent`
  (returns (Intent :type "/Game/Connections/Blueprints/Enums/E_EnemyIntent Enum"))
  (return (cast `/Game/Connections/Blueprints/Enums/E_EnemyIntent` (`KismetMathLibrary.Conv_IntToByte` (`KismetMathLibrary.RandomInteger` (enumcount `/Game/Connections/Blueprints/Enums/E_EnemyIntent`))))))

(fn `GetIntentDescription`
  (returns (Description :type Text))
  (return ""))

(fn `PlayAnim`
  (params (Anim :type "AnimationAsset Object Reference") (Looping :type Boolean))
  (`SkeletalMeshComponent.PlayAnimation` (`self.SkeletalMesh`) Anim Looping))

(fn `UserConstructionScript`
  (`parent.UserConstructionScript`))
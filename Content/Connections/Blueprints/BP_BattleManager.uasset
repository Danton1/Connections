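; Battle manager for a turn-based fight between a player god and an enemy god.
; InitializeBattle supplies the gods' stats components and the HUD, and a short delay after BeginPlay shows and fills the HUD.
; RequestPlayerAction resolves one of six abilities trading Faith, Connection and Followers, then refreshes the HUD and checks for defeat.
; Enemy intent, turn end, alerts and victory/defeat handlers are empty stubs.
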(event `self.ReceiveBeginPlay`
  (`KismetSystemLibrary.Delay` 0.2)
  (`self.StartBattle`))

(fn `Alert`
  (params (Text :type Text)))

(fn `CheckBattleEnd`
  (bind _isdefeated (`/Game/Connections/Blueprints/BP_GodStatsComponent.IsDefeated` (`self.EnemyGodStatsReference`)))
  (if _isdefeated
    (`self.HandleVictory`)
    (else
      (bind _isdefeated_2 (`/Game/Connections/Blueprints/BP_GodStatsComponent.IsDefeated` (`self.PlayerGodStatsReference`)))
      (if _isdefeated_2
        (`self.HandleDefeat`)))))

(fn `EndTurn`)

(fn `GenerateEnemyIntent`)

(fn `HandleDefeat`)

(fn `HandleVictory`)

(fn `InitializeBattle`
  (params (Player :type "/Game/Connections/Blueprints/Characters/BP_BattlePlayer Object Reference") (Enemy :type "/Game/Connections/Blueprints/Characters/BP_EnemyGod Object Reference") (HUD :type "/Game/Connections/Blueprints/UI/WBP_AbilityHUD Object Reference") (PlayerGod :type "/Game/Connections/Blueprints/Characters/BP_PlayerGod Object Reference"))
  (set `self.PlayerRef` Player)
  (bind _output_get (set `self.EnemyRef` Enemy))
  (set `self.EnemyGodStatsReference` (`/Game/Connections/Blueprints/Characters/BP_EnemyGod.BP_GodStatsComponent` _output_get))
  (set `self.AbilityHUD` HUD)
  (bind _output_get_2 (set `self.PlayerGodRef` PlayerGod))
  (set `self.PlayerGodStatsReference` (`/Game/Connections/Blueprints/Characters/BP_PlayerGod.BP_GodStatsComponent` _output_get_2)))

(fn `RequestPlayerAction`
  (params (Action :type "/Game/Connections/Blueprints/Enums/E_GodAction Enum" :default "NewEnumerator0"))
  (if (not (`self.IsResolvingTurn`))
    (`self.ResolvePlayerAction` Action)
    (`self.UpdateHUD`)
    (`self.CheckBattleEnd`)
    (`self.GenerateEnemyIntent`)
    (`self.ResolveEnemyIntent`)
    (`self.UpdateHUD`)
    (`self.CheckBattleEnd`)
    (`self.EndTurn`)))

(fn `ResolveEnemyIntent`)

(fn `ResolvePlayerAction`
  (params (Action :type "/Game/Connections/Blueprints/Enums/E_GodAction Enum" :default "NewEnumerator0"))
  (bind _playergodstatsreference (`self.PlayerGodStatsReference`))
  (bind _playergodstatsreference_2 (`self.PlayerGodStatsReference`))
  (bind _enemygodstatsreference (`self.EnemyGodStatsReference`))
  (bind _playergodstatsreference_3 (`self.PlayerGodStatsReference`))
  (bind _playergodstatsreference_4 (`self.PlayerGodStatsReference`))
  (bind _enemygodstatsreference_2 (`self.EnemyGodStatsReference`))
  (bind _playergodstatsreference_5 (`self.PlayerGodStatsReference`))
  (bind _returnvalue (+ (`/Game/Connections/Blueprints/BP_GodStatsComponent.DivinePower` _playergodstatsreference_4) 8))
  (`KismetSystemLibrary.PrintString` (`|GetEnumeratorNameAsString` Action))
  (switch `/Game/Connections/Blueprints/Enums/E_GodAction` Action
    (:`NewEnumerator0`
      (`/Game/Connections/Blueprints/BP_GodStatsComponent.AddFaith` _playergodstatsreference_2 6)
      (`/Game/Connections/Blueprints/BP_GodStatsComponent.AddConnection` _playergodstatsreference_2 10))
    (:`NewEnumerator1`
      (bind _successful (`/Game/Connections/Blueprints/BP_GodStatsComponent.SpendFaith` _playergodstatsreference_4 3))
      (if _successful
        (`/Game/Connections/Blueprints/BP_GodStatsComponent.TakeFollowerDamage` _enemygodstatsreference_2 _returnvalue)
        (`/Game/Connections/Blueprints/BP_GodStatsComponent.RemoveConnection` _enemygodstatsreference_2 (* _returnvalue 1.5))
        (else
          (`self.Alert` "Not enough Faith"))))
    (:`NewEnumerator2`
      (bind _successful_2 (`/Game/Connections/Blueprints/BP_GodStatsComponent.SpendFaith` _playergodstatsreference_3 5))
      (if _successful_2
        (`/Game/Connections/Blueprints/BP_GodStatsComponent.TakeFollowerDamage` _enemygodstatsreference 6)
        (`/Game/Connections/Blueprints/BP_GodStatsComponent.RemoveConnection` _enemygodstatsreference 10)
        (`/Game/Connections/Blueprints/BP_GodStatsComponent.RemoveFollowers` _enemygodstatsreference 6)
        (`/Game/Connections/Blueprints/BP_GodStatsComponent.AddFollowers` _playergodstatsreference_3 0)
        (else
          (`self.Alert` "Not enough Faith"))))
    (:`NewEnumerator3`
      (`/Game/Connections/Blueprints/BP_GodStatsComponent.SetDefending` (`self.PlayerGodStatsReference`) true))
    (:`NewEnumerator4`
      (`/Game/Connections/Blueprints/BP_GodStatsComponent.RemoveFollowers` _playergodstatsreference 8)
      (`/Game/Connections/Blueprints/BP_GodStatsComponent.AddFaith` _playergodstatsreference 12))
    (:`NewEnumerator5`
      (bind _successful_3 (`/Game/Connections/Blueprints/BP_GodStatsComponent.SpendConnection` _playergodstatsreference_5 (`/Game/Connections/Blueprints/BP_GodStatsComponent.MiracleCost` _playergodstatsreference_5)))
      (if _successful_3
        (`/Game/Connections/Blueprints/BP_GodStatsComponent.TakeFollowerDamage` (`self.EnemyGodStatsReference`) (* (`/Game/Connections/Blueprints/BP_GodStatsComponent.DivinePower` _playergodstatsreference_5) 10))
        (else
          (`self.Alert` "Not enough Connection"))))))

(fn `SetNamesHUD`
  (bind _abilityhud (`self.AbilityHUD`))
  (set `TextBlock.Text` (`/Game/Connections/Blueprints/BP_GodStatsComponent.GodName` (`self.PlayerGodStatsReference`)) (`/Game/Connections/Blueprints/UI/WBP_AbilityHUD.GodName` _abilityhud))
  (set `TextBlock.Text` (`/Game/Connections/Blueprints/BP_GodStatsComponent.GodName` (`self.EnemyGodStatsReference`)) (`/Game/Connections/Blueprints/UI/WBP_AbilityHUD.EnemyName` _abilityhud)))

(fn `StartBattle`
  (set `/Game/Connections/Blueprints/Characters/BP_BattlePlayer.BattleManagerReference` self (`self.PlayerRef`))
  (`UserWidget.AddToViewport` (`self.AbilityHUD`) 0)
  (`self.SetNamesHUD`)
  (`self.UpdateHUD`))

(fn `UpdateHUD`
  (bind _abilityhud (`self.AbilityHUD`))
  (bind _playergodstatsreference (`self.PlayerGodStatsReference`))
  (bind _enemygodstatsreference (`self.EnemyGodStatsReference`))
  (set `TextBlock.Text` (`KismetTextLibrary.Conv_IntToText` (`/Game/Connections/Blueprints/BP_GodStatsComponent.Faith` _playergodstatsreference)) (`/Game/Connections/Blueprints/UI/WBP_AbilityHUD.GodFaith` _abilityhud))
  (set `TextBlock.Text` (`KismetTextLibrary.Conv_IntToText` (`/Game/Connections/Blueprints/BP_GodStatsComponent.Connection` _playergodstatsreference)) (`/Game/Connections/Blueprints/UI/WBP_AbilityHUD.GodConnection` _abilityhud))
  (set `TextBlock.Text` (`KismetTextLibrary.Conv_IntToText` (`/Game/Connections/Blueprints/BP_GodStatsComponent.Health` _playergodstatsreference)) (`/Game/Connections/Blueprints/UI/WBP_AbilityHUD.GodHP` _abilityhud))
  (set `TextBlock.Text` (`KismetTextLibrary.Conv_IntToText` (`/Game/Connections/Blueprints/BP_GodStatsComponent.Followers` _playergodstatsreference)) (`/Game/Connections/Blueprints/UI/WBP_AbilityHUD.GodFollowers` _abilityhud))
  (set `TextBlock.Text` (`KismetTextLibrary.Conv_IntToText` (`/Game/Connections/Blueprints/BP_GodStatsComponent.Health` _enemygodstatsreference)) (`/Game/Connections/Blueprints/UI/WBP_AbilityHUD.EnemyHP` _abilityhud))
  (set `TextBlock.Text` (`KismetTextLibrary.Conv_IntToText` (`/Game/Connections/Blueprints/BP_GodStatsComponent.Followers` _enemygodstatsreference)) (`/Game/Connections/Blueprints/UI/WBP_AbilityHUD.EnemyFollowers` _abilityhud))
  (set `TextBlock.Text` (`KismetTextLibrary.Conv_IntToText` (`/Game/Connections/Blueprints/BP_GodStatsComponent.Faith` _enemygodstatsreference)) (`/Game/Connections/Blueprints/UI/WBP_AbilityHUD.EnemyFaith` _abilityhud))
  (set `TextBlock.Text` (`KismetTextLibrary.Conv_IntToText` (`/Game/Connections/Blueprints/BP_GodStatsComponent.Connection` _enemygodstatsreference)) (`/Game/Connections/Blueprints/UI/WBP_AbilityHUD.EnemyConnection` _abilityhud)))

(fn `UserConstructionScript`)